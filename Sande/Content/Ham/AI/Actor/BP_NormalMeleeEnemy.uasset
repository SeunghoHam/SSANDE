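; BP_NormalMeleeEnemy is an AI enemy actor for a basic melee opponent, supplying its attack, range and movement-speed behavior.
; EnemyAttack is a placeholder that prints a debug message, then triggers a delayed event that signals attack end through CallOnAttackEnd.
; SetMovemenetSpeed maps movement type to walk speed, and GetIdealRange returns fixed attack and defend radii.
; SetTarget only prints a debug message.
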(event Custom|AttackDelay
  (Utilities|FlowControl|Delay 1.0)
  (Default|CallCallonAttackEnd))

(event EventBeginPlay)

(event Collision|EventActorBeginOverlap
  (params (OtherActor :type Actor%20Object%20Reference)))

(event EventTick
  (params (DeltaSeconds :type Float%20%28single-precision%29)))

(fn ConstructionScript)

(fn SetTarget
  (Development|PrintString "[Enemy] Set Target"))

(fn EnemyAttack
  (Development|PrintString "[BP_Enemy] Attack" true true "(R=0.000000,G=1.000000,B=0.022493,A=1.000000)")
  (CallFunction|AttackDelay))

(fn GetIdealRange
  (return 1.5e+02 3e+02))

(fn SetMovemenetSpeed
  (params (MoveType :type E_MovementSpeed%20Enum :default "NewEnumerator0"))
  (bind _output_get (Variables|/Script/Engine.CharacterMovementComponent|SetMaxWalkSpeed (Variables|Character|GetCharacterMovement) (Utilities|Select :Index MoveType :NewEnumerator0 0.0 :NewEnumerator1 1e+02 :NewEnumerator2 2e+02)))
  (return _output_get))