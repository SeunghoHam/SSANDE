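; BP_FXTest is a short-lived test actor that shows a widget component facing the player camera, then destroys itself.
; BeginPlay caches the player camera manager and destroys the actor after a two-second delay.
; Each Tick, while the camera is valid, the widget's world rotation is set from the normalized actor-to-camera vector, giving a billboard effect.
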(event EventBeginPlay
  (Variables|Default|SetCamera (Game|GetPlayerCameraManager 0))
  (Utilities|FlowControl|Delay 2.0)
  (Actor|DestroyActor))

(event Collision|EventActorBeginOverlap
  (params (OtherActor :type Actor%20Object%20Reference)))

(event EventTick
  (params (DeltaSeconds :type Float%20%28single-precision%29))
  (Utilities|IsValid (Variables|Default|GetCamera)
    (:Is%20Valid
      (Transformation|SetWorldRotation (Variables|Default|GetWidget) (Math|Conversions|RotationFromXVector (Math|Vector|Normalize (- (Transformation|GetActorLocation (Variables|Default|GetCamera)) (Transformation|GetActorLocation)))) false false))))

(fn ConstructionScript)